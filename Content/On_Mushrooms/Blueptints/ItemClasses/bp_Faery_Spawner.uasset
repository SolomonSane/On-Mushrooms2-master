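; Faery spawner actor that spawns a random class from SpawnedClasses at its own transform on BeginPlay.
; When My_TopDownCharacter overlaps its Sphere, it tries to add ItemClass and Amount to the character's CageRef.
; A partial add leaves the remainder in Amount.
; A full add destroys the spawned actor and spawns another random one after a short delay, without resetting Amount or updating ItemClass.
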(event `self.ReceiveBeginPlay`
  (`self.SpawnFaery`))

(event `self.Sphere.OnComponentBeginOverlap`
  (params (OverlappedComponent :type "PrimitiveComponent Object Reference") (OtherActor :type "Actor Object Reference") (OtherComp :type "PrimitiveComponent Object Reference") (OtherBodyIndex :type Integer) (bFromSweep :type Boolean) (SweepResult :type "HitResult Structure (by ref)"))
  (bind _masteritem (`self.MasterItem`))
  (bind _asmy_top_down_character (cast `/Game/On_Mushrooms/Character/My_TopDownCharacter` OtherActor))
  (bind _cageref (`/Game/On_Mushrooms/Character/My_TopDownCharacter.CageRef` _asmy_top_down_character))
  (`/Engine/EditorBlueprintResources/StandardMacros.IsValid` _cageref
    (:`Is Valid`
      (bind (_success_ _rest) (`/Game/On_Mushrooms/Blueptints/UI/bp_Cage.- Add Item` _cageref (`self.Item Class`) (`self.Amount`)))
      (if _success_
        (if (> _rest 0)
          (set `self.Amount` _rest)
          (else
            (`/Engine/EditorBlueprintResources/StandardMacros.IsValid` _masteritem
              (:`Is Valid`
                (`self.K2_DestroyActor` _masteritem)
                (`KismetSystemLibrary.Delay` 3.0)
                (`self.SpawnFaery`)))))))))

(fn `SpawnFaery`
  (bind _returnvalue (`|SpawnActorFromClass` (`KismetArrayLibrary.Array_Random` (`self.spawned_classes`)) (`self.GetTransform`) "AlwaysSpawn" "OverrideRootScale" null null))
  (set `self.MasterItem` _returnvalue))

(fn `UserConstructionScript`)